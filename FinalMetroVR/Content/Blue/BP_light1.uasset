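; BP_light1 is a flickering point light with a sound effect.
; From BeginPlay, a looping Delay chain waits a random long interval, then cuts the light's intensity to zero.
; If Power is true, audio plays for a brief random blackout, then stops as the light returns and the loop repeats.
; If Power is false at that check, the light stays dark and the loop ends.
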(event `self.ReceiveBeginPlay`
  (bind _pointlightcomponent (`self.PointLightComponent`))
  (bind _audio (`self.Audio`))
  (`KismetSystemLibrary.Delay` (`KismetMathLibrary.RandomFloatInRange` 1.0 100.0) :!label _label)
  (`LightComponent.SetIntensity` _pointlightcomponent 0.0)
  (if (`self.Power`)
    (`AudioComponent.Play` _audio 0.0)
    (`KismetSystemLibrary.Delay` (`KismetMathLibrary.RandomFloatInRange` 0.01 0.1))
    (`AudioComponent.Stop` _audio)
    (`LightComponent.SetIntensity` _pointlightcomponent 200.0)
    (goto _label)))

(fn `UserConstructionScript`)