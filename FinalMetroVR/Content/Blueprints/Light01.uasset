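; Light01 is a flickering point light actor with electric spark audio.
; On BeginPlay it loops: after a Tempo delay it sets the light to zero and, while Power is true, plays the sparks sound.
; After a brief random delay it stops the sound, restores intensity and repeats.
; When Power is false the loop ends with the light off.
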(event `self.ReceiveBeginPlay`
  (bind _pointlight (`self.PointLight`))
  (bind _396470__kev_durr__electric_sparks (`self.396470__kev-durr__electric-sparks`))
  (`KismetSystemLibrary.Delay` (`self.tempo`) :!label _label)
  (`LightComponent.SetIntensity` _pointlight 0.0)
  (if (`self.power`)
    (`AudioComponent.Play` _396470__kev_durr__electric_sparks 0.0)
    (`KismetSystemLibrary.Delay` (`KismetMathLibrary.RandomFloatInRange` 0.01 0.1))
    (`AudioComponent.Stop` _396470__kev_durr__electric_sparks)
    (`LightComponent.SetIntensity` _pointlight 300.0)
    (goto _label)))

(event `self.ReceiveTick`
  (params (DeltaSeconds :type "Float (single-precision)")))

(fn `UserConstructionScript`)